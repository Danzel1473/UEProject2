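; BP_DamageReciever tracks health and stamina for whatever takes damage, starting both at their maximums on BeginPlay.
; RecieveDamage subtracts damage from health and, at zero or below, clamps it to zero and calls OnDead, with no guard against repeat calls.
; UseStamina reduces stamina without clamping.
; GetHPPercent and GetStaminaPercent return each value as a fraction of its maximum.
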(event `self.ReceiveBeginPlay`
  (set `self.HealthPower` (`self.MaxHealthPower `))
  (set `self.Stamina` (`self.MaxStamina`)))

(event `RecieveDamage`
  (params (Damage :type "Float (double-precision)"))
  ;[1 1 1] 대미지 처리 공식
  (set `self.HealthPower` (- (`self.HealthPower`) Damage))
  (if (<= (`self.HealthPower`) 0.0)
    (set `self.HealthPower` 0.0)
    (`self.OnDead`)))

(event `UseStamina`
  (params (Stamina :type "Float (double-precision)"))
  (set `self.Stamina` (- (`self.Stamina`) Stamina)))

(fn `GetHPPercent`
  (returns (Percent :type "Float (double-precision)"))
  (return (/ (`self.HealthPower`) (`self.MaxHealthPower `))))

(fn `GetStaminaPercent`
  (returns (Percent :type "Float (double-precision)"))
  (return (/ (`self.Stamina`) (`self.MaxStamina`))))