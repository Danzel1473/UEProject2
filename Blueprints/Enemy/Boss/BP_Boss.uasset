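; Boss enemy character that chases and attacks the player, with its name and health shown on the main UI.
; SetState mirrors the state to the AI blackboard and sets walk speed, with Dead as terminal.
; Pawn sensing starts the chase, and an attack collider toggled by check events damages non-invincible players.
; Incoming damage feeds DamageReciever, camera shake, hit sound and HP bar, and its death event disables collision.
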(event `OnAttackCheckBegin`
  (`PrimitiveComponent.SetCollisionEnabled` (`self.AttackCollision`) "QueryOnly"))

(event `OnAttackCheckEnd`
  (`PrimitiveComponent.SetCollisionEnabled` (`self.AttackCollision`) "NoCollision"))

(event `self.ReceiveBeginPlay`
  (add `/Game/Blueprints/BP_DamageReciever.OnDead` (`self.DamageReciever`) (delegate `OnDead`))
  (`PrimitiveComponent.SetCollisionEnabled` (`self.AttackCollision`) "NoCollision"))

(event `OnDead`
  (`self.SetState` "NewEnumerator3")
  (`PrimitiveComponent.SetCollisionEnabled` (`self.CapsuleComponent`) "NoCollision")
  (`PrimitiveComponent.SetCollisionEnabled` (`self.Mesh`) "NoCollision"))

(event `SetState`
  (params (`New State` :type "/Game/Blueprints/Enemy/Boss/E_Boss Enum" :default "NewEnumerator0"))
  (if (`|EnumInequality` (`self.State`) "NewEnumerator3")
    (if (`|EnumInequality` (`self.State`) `New State`)
      (bind _output_get (set `self.State` `New State`))
      (`BlackboardComponent.SetValueAsEnum` (`AIBlueprintHelperLibrary.GetBlackboard` (`AIBlueprintHelperLibrary.GetAIController` self)) (`self.StateKey`) _output_get)
      (`|ExecutionSequence`
        (:`then_0`
          (switch `/Game/Blueprints/Enemy/Boss/E_Boss` (`self.State`)
            (:`NewEnumerator0`
              (set `CharacterMovementComponent.MaxWalkSpeed` 200.0 (`self.CharacterMovement`)))
            (:`NewEnumerator1`
              (set `CharacterMovementComponent.MaxWalkSpeed` 400.0 (`self.CharacterMovement`)))
            (:`NewEnumerator2`
              (set `CharacterMovementComponent.MaxWalkSpeed` 0.0 (`self.CharacterMovement`) :!label _label))
            (:`NewEnumerator3`
              (goto _label))))))))

(event `self.ReceiveAnyDamage`
  (params (Damage :type "Float (single-precision)") (DamageType :type "DamageType Object Reference") (InstigatedBy :type "Controller Object Reference") (DamageCauser :type "Actor Object Reference"))
  (`/Game/Blueprints/BP_DamageReciever.RecieveDamage` (`self.DamageReciever`) Damage)
  (`PlayerCameraManager.StartCameraShake` :`self` (`GameplayStatics.GetPlayerCameraManager` 0) :`ShakeClass` "/Game/Blueprints/BP_CameraShake.BP_CameraShake_C")
  (bind _percent (`/Game/Blueprints/BP_DamageReciever.GetHPPercent` (`self.DamageReciever`)))
  (bind _asbp_player_controller (cast `/Game/Blueprints/Player/BP_PlayerController` (`self.GetController` (`GameplayStatics.GetPlayerCharacter` 0))))
  (`/Game/Blueprints/WBP_Main.SetEnemyHPPercent` (`/Game/Blueprints/Player/BP_PlayerController.MainUI` _asbp_player_controller) _percent)
  (`GameplayStatics.PlaySoundAtLocation` "/Game/Sound/hit-flesh-02-266309.hit-flesh-02-266309" (`self.K2_GetActorLocation`) (struct) 1.0 1.0 0.2 null null null null))

(event `self.PawnSensing.OnSeePawn`
  (params (Pawn :type "Pawn Object Reference"))
  (if (`|EnumEquality` (`self.State`) "NewEnumerator0")
    (cast `/Game/Blueprints/Player/BP_Mannequin` Pawn)
    (if (`|EnumInequality` (`self.State`) "NewEnumerator3")
      (`self.SetState` "NewEnumerator1")
      (bind _output_get (set `self.Instigator` Pawn))
      (`BlackboardComponent.SetValueAsObject` (`AIController.Blackboard` (`AIBlueprintHelperLibrary.GetAIController` self)) (`self.TargetPlayerKey`) _output_get)
      (bind _asbp_player_controller (cast `/Game/Blueprints/Player/BP_PlayerController` (`self.GetController` (`GameplayStatics.GetPlayerCharacter` 0))))
      (`/Game/Blueprints/WBP_Main.Boss Name And HPBar Visible` (`/Game/Blueprints/Player/BP_PlayerController.MainUI` _asbp_player_controller) (`self.BossName`)))))

(event `self.AttackCollision.OnComponentBeginOverlap`
  (params (OverlappedComponent :type "PrimitiveComponent Object Reference") (OtherActor :type "Actor Object Reference") (OtherComp :type "PrimitiveComponent Object Reference") (OtherBodyIndex :type Integer) (bFromSweep :type Boolean) (SweepResult :type "HitResult Structure (by ref)"))
  (bind _asbp_mannequin (cast `/Game/Blueprints/Player/BP_Mannequin` OtherActor))
  (if (not (`/Game/Blueprints/Player/BP_Mannequin.Invincibility` _asbp_mannequin))
    (`GameplayStatics.ApplyDamage` OtherActor (`self.Base Damage`) (`self.GetController`) self)
    (`KismetSystemLibrary.PrintString` "Hello")))

(event `AttackCheckBegin`
  (`PrimitiveComponent.SetCollisionEnabled` (`self.AttackCollision`) "QueryOnly"))

(event `AttackCheckEnd`
  (`PrimitiveComponent.SetCollisionEnabled` (`self.AttackCollision`) "NoCollision"))

(fn `TurnToTarget`
  (bind _returnvalue (`GameplayStatics.GetPlayerPawn` 0))
  (bind (_returnvalue_roll _returnvalue_pitch _returnvalue_yaw) (`KismetMathLibrary.BreakRotator` (`KismetMathLibrary.MakeRotFromX` (- (`self.K2_GetActorLocation` _returnvalue) (`self.K2_GetActorLocation`)))))
  (`/Engine/EditorBlueprintResources/StandardMacros.IsValid` _returnvalue
    (:`Is Valid`
      (`self.K2_SetActorRotation` (`KismetMathLibrary.MakeRotator` 0.0 0.0 _returnvalue_yaw)))))

(fn `UserConstructionScript`)